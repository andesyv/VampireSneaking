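; Enemy actor that shows its damage through mesh color and explodes when destroyed.
; On BeginPlay it creates a dynamic material instance for the mesh.
; Each tick it reads blood percentage from the HealthComponent on its EnemyAI_BP controller and sets the ColorIn parameter, with green and blue at one minus that value.
; On destruction it spawns a scaled-up explosion emitter at its location.
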(event `self.ReceiveBeginPlay`
  (bind _returnvalue (`PrimitiveComponent.CreateDynamicMaterialInstance` (`self.Mesh`) 0 null))
  (set `self.Material` _returnvalue))

(event `self.ReceiveTick`
  (params (DeltaSeconds :type "Float (single-precision)"))
  (bind _asenemy_ai_bp (cast `/Game/Blueprints/AIBehavior/EnemyAI_BP` (`self.GetController`)))
  (bind _returnvalue (- 1.0 (`HealthComponent.GetPercentageBlood` (`EnemyAI.HealthComponent` _asenemy_ai_bp))))
  (`MaterialInstanceDynamic.SetVectorParameterValue` (`self.Material`) "ColorIn" (make `LinearColor` 1.0 _returnvalue _returnvalue)))

(event `self.ReceiveDestroyed`
  (`GameplayStatics.SpawnEmitterAtLocation` "/Game/Particles/P_Explosion.P_Explosion" (`self.K2_GetActorLocation`) (struct) (3.0 3.0 3.0)))

(fn `UserConstructionScript`)