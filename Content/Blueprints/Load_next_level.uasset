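; A level transition trigger actor that plays a cutscene when a playable character overlaps it, then loads BetaMap.
; On overlap it clears all widgets, adds a Movie widget for the character's player controller and opens the Transition source on the media player.
; A fixed delay, rather than a playback-finished event, times the level load, which also requires a successful cast to VampireSneakingGameModeBase.
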(event `self.ReceiveActorBeginOverlap`
  (params (OtherActor :type "Actor Object Reference"))
  (bind (_asplayable_character_base _bsuccess) (cast `PlayableCharacterBase` OtherActor :!pure true))
  (bind (_asplayer_controller _bsuccess_2) (cast `PlayerController` (`Pawn.GetController` _asplayable_character_base) :!pure true))
  (if _bsuccess
    (`WidgetLayoutLibrary.RemoveAllWidgets`)
    (if _bsuccess_2
      (bind _returnvalue (`|CreateWidget` "/Game/UI/Movie.Movie_C" _asplayer_controller))
      (`UserWidget.AddToViewport` _returnvalue 0)
      (`MediaPlayer.OpenSource` (`self.mediaplayer`) "/Game/Movies/Transition.Transition")
      (`KismetSystemLibrary.Delay` 115.0)
      (cast `VampireSneakingGameModeBase` (`GameplayStatics.GetGameMode`))
      (`GameplayStatics.OpenLevel` "BetaMap"))))

(fn `UserConstructionScript`)