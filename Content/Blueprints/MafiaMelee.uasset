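; MafiaMelee is an enemy character Blueprint for a melee mafia enemy with a glowing cigarette.
; At BeginPlay it creates a dynamic CigaretteGlow material on the second material slot of its mesh.
; Each tick it casts its controller to EnemyAI_BP and feeds that controller's health component blood percentage into the glow parameter.
; Its Attack function forwards the damage, range and angle variables to MeleeAttack.
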(event `self.ReceiveBeginPlay`
  (bind _returnvalue (`PrimitiveComponent.CreateDynamicMaterialInstance` (`self.Mesh`) 1 "/Game/Materials/CigaretteGlow.CigaretteGlow"))
  (set `self.Material_0` _returnvalue))

(event `self.ReceiveTick`
  (params (DeltaSeconds :type "Float (single-precision)"))
  (bind _asenemy_ai_bp (cast `/Game/Blueprints/AIBehavior/EnemyAI_BP` (`self.GetController`)))
  (`MaterialInstanceDynamic.SetScalarParameterValue` (`self.Material_0`) "GlowPercentage" (`HealthComponent.GetPercentageBlood` (`EnemyAI.HealthComponent` _asenemy_ai_bp))))

(fn `Attack`
  (`self.MeleeAttack` (`self.AttackDamage`) (`self.AttackRange`) (`self.AttackAngle`)))

(fn `UserConstructionScript`)