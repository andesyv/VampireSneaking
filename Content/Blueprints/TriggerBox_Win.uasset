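; TriggerBox_Win is a win trigger that shows the win screen when a playable character overlaps it.
; On overlap with a PlayableCharacterBase, it removes all widgets, then creates a Winscreen widget for that character's player controller and adds it to the viewport.
; After a short delay it casts the game mode to VampireSneakingGameModeBase, but nothing follows that cast.
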(event `self.ReceiveActorBeginOverlap`
  (params (OtherActor :type "Actor Object Reference"))
  (bind (_asplayable_character_base _bsuccess) (cast `PlayableCharacterBase` OtherActor :!pure true))
  (bind (_asplayer_controller _bsuccess_2) (cast `PlayerController` (`Pawn.GetController` _asplayable_character_base) :!pure true))
  (if _bsuccess
    (`WidgetLayoutLibrary.RemoveAllWidgets`)
    (if _bsuccess_2
      (bind _returnvalue (`|CreateWidget` "/Game/UI/Winscreen.Winscreen_C" _asplayer_controller))
      (`UserWidget.AddToViewport` _returnvalue 0)
      (`KismetSystemLibrary.Delay` 2.0)
      (cast `VampireSneakingGameModeBase` (`GameplayStatics.GetGameMode`)))))

(fn `UserConstructionScript`)