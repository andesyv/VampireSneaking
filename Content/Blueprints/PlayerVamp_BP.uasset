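; Player vampire Blueprint that adds HUD setup, eye blinking and a sword-slash attack visual on top of its parent class.
; BeginPlay clears all widgets, creates the default HUD and makes dynamic materials for the eyes and slash sprite.
; A looping timer triggers a timeline that animates the eye material's blink phase.
; Attack calls the parent, then a timeline rotates the slash sprite from its starting yaw and drives its visibility through a material parameter.
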(event `self.ReceiveBeginPlay`
  (bind _attacksprite (`self.AttackSprite`))
  (`parent.ReceiveBeginPlay`)
  (`WidgetLayoutLibrary.RemoveAllWidgets`)
  (bind _returnvalue (`|CreateWidget` "/Game/UI/DefaultHUD.DefaultHUD_C" (`GameplayStatics.GetPlayerController` 0)))
  (`UserWidget.AddToViewport` _returnvalue 0)
  (set `self.StartRelativeRotation` (`SceneComponent.RelativeRotation` _attacksprite))
  (bind _returnvalue_2 (`PrimitiveComponent.CreateDynamicMaterialInstance` _attacksprite 0 "/Game/Materials/SwordSlashMat.SwordSlashMat"))
  (set `self.PlaneMaterial` _returnvalue_2)
  ;[1 1 1] Initiate blinking timer
  (bind _returnvalue_3 (`PrimitiveComponent.CreateDynamicMaterialInstance` (`self.Mesh`) 2 "/Game/Materials/VampireEyes.VampireEyes"))
  (set `self.EyesMaterial` _returnvalue_3)
  (`KismetSystemLibrary.K2_SetTimerDelegate` (delegate `InitiateBlinking`) 8.0 true))

(event `InitiateBlinking`
  ;[1 1 1] Blink
  (bind (_direction _animationphase) (`Timeline|BlinkingTimeline` :!via `PlayFromStart`)
    (:`Update`
      (`MaterialInstanceDynamic.SetScalarParameterValue` (`self.EyesMaterial`) "AnimationPhase" _animationphase))))

(event `self.Attack`
  (`parent.Attack`)
  (bind (_direction _materialvisibility _rotation) (`Timeline|AttackTimeline` :!via `PlayFromStart`)
    (:`Update`
      (`SceneComponent.K2_SetRelativeRotation` (`self.AttackSprite`) (`KismetMathLibrary.MakeRotator` (.x _rotation) (.y _rotation) (+ (.z _rotation) (.yaw (`self.StartRelativeRotation`)))) false false)
      (`MaterialInstanceDynamic.SetScalarParameterValue` (`self.PlaneMaterial`) "Multiplier" _materialvisibility))))

(fn `UserConstructionScript`)